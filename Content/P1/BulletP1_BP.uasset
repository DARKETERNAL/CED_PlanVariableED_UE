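; BulletP1_BP is a bullet actor that destroys targets sharing its color.
; On a static mesh hit, it casts the other actor to TargetP1_BP and destroys it if the Color values match.
; The bullet then destroys itself after any hit, whether or not the target matches.
; BeginPlay also starts a delay that destroys the bullet after AutoDestroyTime.
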(event OnComponentHit(StaticMeshComponent)
  (params (HitComponent :type Primitive%20Component%20Object%20Reference) (OtherActor :type Actor%20Object%20Reference) (OtherComp :type Primitive%20Component%20Object%20Reference) (NormalImpulse :type Vector :default "0, 0, 0") (Hit :type Hit%20Result%20Structure%20%28by%20ref%29))
  (Utilities|FlowControl|Sequence
    (:then_0
      (bind _astarget_p1_bp (Utilities|Casting|CastToTargetP1_BP OtherActor))
      (if (Utilities|Enum|Equal(Enum) (Variables|/Game/P1/TargetP1_BP.TargetP1_BP_C|GetColor _astarget_p1_bp) (Variables|Default|GetColor))
        (Actor|DestroyActor OtherActor)))
    (:then_1
      (Actor|DestroyActor))))

(event EventBeginPlay
  (Utilities|FlowControl|Delay (Variables|Default|GetAutoDestroyTime))
  (Actor|DestroyActor))

(fn ConstructionScript)