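; Target spawner actor that launches red or yellow targets, built to fire repeatedly on a timer.
; BeginPlay starts a looping SpawnRate timer, presumably bound to SpawnNextTarget.
; SpawnNextTarget randomly picks RedTargetP1_BP or YellowTargetP1_BP and spawns it at the spawner's location with a fixed rotation.
; It then casts to TargetP1_BP and pushes its mesh along the spawner's forward vector with a ShootForce-scaled physics force.
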(event EventBeginPlay
  (Utilities|Time|SetTimerbyEvent (EventDispatchers|CreateEvent :!event SpawnNextTarget) (Variables|Default|GetSpawnRate) true))

(fn ConstructionScript)

(fn SpawnNextTarget
  (bind _returnvalue (Game|SpawnActorfromClass (select (Math|Random|RandomBool) "/Game/P1/RedTargetP1_BP.RedTargetP1_BP_C" "/Game/P1/YellowTargetP1_BP.YellowTargetP1_BP_C") (Math|Transform|MakeTransform (Transformation|GetActorLocation) "90.000000, 0, 0" "1,1,1") "Undefined" 0 0))
  (bind _astarget_p1_bp (Utilities|Casting|CastToTargetP1_BP _returnvalue))
  (Physics|AddForce (Variables|/Script/Engine.StaticMeshActor|GetStaticMeshComponent _astarget_p1_bp) (* (Transformation|GetActorForwardVector) (Variables|Default|GetShootForce)) "None" false))